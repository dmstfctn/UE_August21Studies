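; Parametric fridge actor that builds a body of configurable length and stocks its shelves with randomized bottle displays.
; The construction script tiles FridgeBody meshes by SectionCount, moves the right end piece into place and derives the shelf length.
; On BeginPlay or a G key press, it destroys earlier BottleSet actors and fills six shelf rows with attached sets of random width, using remaining space to cap them.
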(event `Key|G`
  (params (Key :type "Key Structure"))
  (bind _shelffilled (`self.ShelfFilled`))
  (bind _spawnedbottlesets (`self.SpawnedBottleSets`))
  (bind _returnvalue (`KismetMathLibrary.Conv_IntToDouble` (* (`KismetMathLibrary.RandomIntegerInRange` 2 8) 10)))
  (bind _returnvalue_2 (- (- (`self.ShelfLength`) (`self.ShelfEdgeSpacing`)) (`self.ShelfFilled`)))
  (:`Pressed`
    (for (_array_element _array_index) _spawnedbottlesets :!label _label
      (`self.K2_DestroyActor` _array_element))
    (`KismetArrayLibrary.Array_Clear` _spawnedbottlesets)
    (for _index (range 6)
      (set `self.ShelfFilled` (`KismetSystemLibrary.MakeLiteralDouble` (`self.ShelfEdgeSpacing`)))
      (while (< (`self.ShelfFilled`) (- (`self.ShelfLength`) (`self.ShelfEdgeSpacing`)))
        (bind _output_get (set `self.CurrentBottleBoxWidth` (select `bool` (> _returnvalue _returnvalue_2) :`false` _returnvalue :`true` _returnvalue_2)))
        (bind _returnvalue_3 (`|SpawnActorFromClass` "/Game/AugustStudies/blueprints/BottleSet.BottleSet_C" (`KismetMathLibrary.MakeTransform` (`KismetMathLibrary.MakeVector` -12.0 (* _shelffilled -1.0) (+ (* (`KismetMathLibrary.Conv_IntToDouble` _index) 25.700001) 34.5))) "Undefined" "OverrideRootScale" null (* _output_get 0.5) 15.0 0 null))
        (`self.K2_AttachToActor` _returnvalue_3 (`ActorComponent.GetOwner` (`self.DefaultSceneRoot`)) "None" "KeepRelative" "KeepRelative" "KeepRelative" false)
        (`KismetArrayLibrary.Array_Add` (`self.SpawnedBottleSets`) _returnvalue_3)
        (set `self.ShelfFilled` (+ _shelffilled _output_get))))))

(event `self.ReceiveBeginPlay`
  (`self.EnableInput` (`GameplayStatics.GetPlayerController` 0))
  (goto _label))

(fn `UserConstructionScript`
  (bind _returnvalue (- (`self.SectionCount`) 1))
  (`|ExecutionSequence`
    (:`then_0`
      (set `self.ShelfLength` (* (`self.SectionWidth`) (`self.SectionCount`))))
    (:`then_1`
      (for _index (range (+ _returnvalue 1))
        (bind _returnvalue_2 (`AddComponent|NODE_AddStaticMeshComponent-0` :`bManualAttachment` true))
        (`SceneComponent.K2_AttachToComponent` _returnvalue_2 (`self.DefaultSceneRoot`) "None" "KeepRelative" "KeepRelative" "KeepRelative" false)
        (`StaticMeshComponent.SetStaticMesh` _returnvalue_2 (`self.FridgeBody`))
        (`SceneComponent.K2_SetRelativeLocation` _returnvalue_2 (`KismetMathLibrary.MakeVector` 0.0 (* (`KismetMathLibrary.Conv_IntToDouble` _index) (* (`self.SectionWidth`) -1.0))) false true))
      ;[0 0 0] Position right hand side of fridge
      (`SceneComponent.K2_SetRelativeLocation` (`self.fridge_right`) (`KismetMathLibrary.MakeVector` 0.0 (+ (* (`KismetMathLibrary.Conv_IntToDouble` _returnvalue) (* (`self.SectionWidth`) -1.0)) 1.0)) false true))))