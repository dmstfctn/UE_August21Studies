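; Post-process actor that switches the view between depth and label render styles.
; The construction script creates dynamic instances of both materials, applies editor-set depth range and label count, and puts the chosen initial mode in the blendables array.
; BeginPlay enables player input and reapplies both parameters.
; P toggles post-processing, while L and K swap in the depth and label materials respectively.
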(event `self.ReceiveBeginPlay`
  (`|ExecutionSequence`
    (:`then_0`
      (`self.EnableInput` (`GameplayStatics.GetPlayerController` 0)))
    (:`then_1`
      (`MaterialInstanceDynamic.SetScalarParameterValue` (`self.DynamicDepthPPMat`) "MaxDepth" (`self.DepthRange`))
      (`MaterialInstanceDynamic.SetScalarParameterValue` (`self.DynamicLabelPPMat`) "MaxLabelCount" (`KismetMathLibrary.Conv_ByteToDouble` (`self.MaxLabelCount`))))))

(event `Key|P`
  (params (Key :type "Key Structure"))
  ;[0 0 0 1 12] Enable/Disable PostProcessing on P
  (:`Pressed`
    (bind _output_get (set `self.PostProcessingIsActive` (not (`self.PostProcessingIsActive`))))
    (set `PostProcessComponent.bEnabled` _output_get (`self.PostProcess`))))

(event `Key|L`
  (params (Key :type "Key Structure"))
  ;[0 0 0] Toggle Different Materials/Styles on K and L
  (:`Pressed`
    (`KismetArrayLibrary.Array_Set` (`.Array` (break `WeightedBlendables` (`.WeightedBlendables` (break `PostProcessSettings` (`PostProcessComponent.Settings` (`self.PostProcess`)))))) 0 (make `WeightedBlendable` 1.0 (`self.DynamicDepthPPMat`)))))

(event `Key|K`
  (params (Key :type "Key Structure"))
  ;[0 0 0] Toggle Different Materials/Styles on K and L
  (:`Pressed`
    (`KismetArrayLibrary.Array_Set` (`.Array` (break `WeightedBlendables` (`.WeightedBlendables` (break `PostProcessSettings` (`PostProcessComponent.Settings` (`self.PostProcess`)))))) 0 (make `WeightedBlendable` 1.0 (`self.DynamicLabelPPMat`)))))

(fn `UserConstructionScript`
  (`|ExecutionSequence`
    (:`then_0`
      ;[0 0 0 1 12] Set PP Volume to active/inactive based on editor panel settings
      (set `PostProcessComponent.bEnabled` (`self.PostProcessingIsActive`) (`self.PostProcess`)))
    (:`then_1`
      ;[0 0 0 1 12] Initialise Dynamic Material Instances for each render style
      (bind _returnvalue (`KismetMaterialLibrary.CreateDynamicMaterialInstance` "/Game/AugustStudies/post_process/ppm_depth.ppm_depth"))
      (set `self.DynamicDepthPPMat` _returnvalue)
      (bind _returnvalue_2 (`KismetMaterialLibrary.CreateDynamicMaterialInstance` "/Game/AugustStudies/post_process/ppm_labels.ppm_labels"))
      (set `self.DynamicLabelPPMat` _returnvalue_2))
    (:`then_2`
      ;[0 0 0 1 12] Set active render style (depth as default)
      (`KismetArrayLibrary.Array_Set` (`.Array` (break `WeightedBlendables` (`.WeightedBlendables` (break `PostProcessSettings` (`PostProcessComponent.Settings` (`self.PostProcess`)))))) 0 (make `WeightedBlendable` 1.0 (select `/Game/AugustStudies/blueprints/EPostProcessTypes` (`self.InitialMode`) :`NewEnumerator0` (`self.DynamicDepthPPMat`) :`NewEnumerator1` (`self.DynamicLabelPPMat`)))))
    (:`then_3`
      ;[0 0 0 1 12] Se Render Mode Values based on editor panel settings
      (`MaterialInstanceDynamic.SetScalarParameterValue` (`self.DynamicDepthPPMat`) "MaxDepth" (`self.DepthRange`))
      (`MaterialInstanceDynamic.SetScalarParameterValue` (`self.DynamicLabelPPMat`) "MaxLabelCount" (`KismetMathLibrary.Conv_ByteToDouble` (`self.MaxLabelCount`))))))