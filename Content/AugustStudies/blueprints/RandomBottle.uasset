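; Bottle actor that randomises its mesh and colours, or derives them repeatably from a positive BottleTypeID.
; The construction script creates dynamic material instances for liquid, plastic, label and lid.
; BeginPlay seeds a random stream, picks the mesh and custom-depth stencil by modulo, and tints liquid, label and lid from the stream, keeping plastic white.
; Without a positive ID, seed, mesh and stencil each use a separate random roll.
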(event `self.ReceiveBeginPlay`
  (bind _listofbottlemeshes (`self.ListOfBottleMeshes`))
  (bind _bottlemesh (`self.BottleMesh`))
  (bind _bottletypeid (`self.BottleTypeID`))
  (bind _randomsource (`self.RandomSource`))
  (bind _returnvalue (select `int` (`KismetMathLibrary.Clamp` _bottletypeid 0 1) :`0` (`KismetMathLibrary.RandomInteger` 100000) :`1` _bottletypeid))
  (`KismetMathLibrary.SetRandomStreamSeed` _randomsource _returnvalue)
  (`StaticMeshComponent.SetStaticMesh` (`self.BottleMesh`) (`|GetArrayItem` _listofbottlemeshes (mod _returnvalue (`KismetArrayLibrary.Array_Length` _listofbottlemeshes))))
  (`PrimitiveComponent.SetRenderCustomDepth` _bottlemesh true)
  (`PrimitiveComponent.SetCustomDepthStencilValue` _bottlemesh (mod _returnvalue 20))
  (`MaterialInstanceDynamic.SetVectorParameterValue` (`self.DynamicLiquid`) "LiquidColour" (`KismetMathLibrary.MakeColor` (`KismetMathLibrary.RandomFloatInRangeFromStream` 0.2 0.9 _randomsource) (`KismetMathLibrary.RandomFloatInRangeFromStream` 0.2 0.9 _randomsource) (`KismetMathLibrary.RandomFloatInRangeFromStream` 0.2 0.9 _randomsource)))
  (`MaterialInstanceDynamic.SetVectorParameterValue` (`self.DynamicBottle`) "PlasticColour" (`KismetMathLibrary.MakeColor` 1.0 1.0 1.0))
  (`MaterialInstanceDynamic.SetVectorParameterValue` (`self.DynamicLabel`) "LabelColour" (`KismetMathLibrary.MakeColor` (`KismetMathLibrary.RandomFloatInRangeFromStream` 0.2 0.9 _randomsource) (`KismetMathLibrary.RandomFloatInRangeFromStream` 0.2 0.9 _randomsource) (`KismetMathLibrary.RandomFloatInRangeFromStream` 0.2 0.9 _randomsource)))
  (`MaterialInstanceDynamic.SetVectorParameterValue` (`self.DynamicLid`) "LidColour" (`KismetMathLibrary.MakeColor` (`KismetMathLibrary.RandomFloatInRangeFromStream` 0.2 0.9 _randomsource) (`KismetMathLibrary.RandomFloatInRangeFromStream` 0.2 0.9 _randomsource) (`KismetMathLibrary.RandomFloatInRangeFromStream` 0.2 0.9 _randomsource))))

(fn `UserConstructionScript`
  (bind _bottlemesh (`self.BottleMesh`))
  (bind _returnvalue (`PrimitiveComponent.CreateDynamicMaterialInstance` _bottlemesh 0 "/Game/AugustStudies/materials/m_bottle_liquid.m_bottle_liquid" "None"))
  (set `self.DynamicLiquid` _returnvalue)
  (bind _returnvalue_2 (`PrimitiveComponent.CreateDynamicMaterialInstance` _bottlemesh 3 "/Game/AugustStudies/materials/m_bottle_plastic.m_bottle_plastic" "None"))
  (set `self.DynamicBottle` _returnvalue_2)
  (bind _returnvalue_3 (`PrimitiveComponent.CreateDynamicMaterialInstance` _bottlemesh 2 "/Game/AugustStudies/materials/m_bottle_label.m_bottle_label" "None"))
  (set `self.DynamicLabel` _returnvalue_3)
  (bind _returnvalue_4 (`PrimitiveComponent.CreateDynamicMaterialInstance` _bottlemesh 1 "/Game/AugustStudies/materials/m_bottle_lid.m_bottle_lid" "None"))
  (set `self.DynamicLid` _returnvalue_4))