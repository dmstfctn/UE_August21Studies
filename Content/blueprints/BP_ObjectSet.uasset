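; Procedural set-dressing actor that fills a box area with rows of randomly picked static meshes, such as stacked goods.
; The construction script repeatedly spawns seeded grids along Y until space runs out, storing each mesh as a cell in AllCells.
; Density drives stacking, hiding cells above empty ones, while Variance jitters position and yaw.
; At runtime, R randomises cell visibility and T reveals cells one by one on a looping timer.
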(event `self.ReceiveBeginPlay`
  (`self.EnableInput` (`GameplayStatics.GetPlayerControllerFromID` 0)))

(event `Key|R`
  (params (Key :type "Key Structure"))
  (bind _allcells (`self.AllCells`))
  ;[0 0 0] Randomises visibility of objects. This is a permanent/stored change during play
  (:`Pressed`
    (for (_array_element _array_index) _allcells
      (bind _structout (setmembers `/Game/blueprints/SObjectSetCell` :`StructRef` _array_element :`Visible` (`KismetMathLibrary.RandomBool`)))
      (`KismetArrayLibrary.Array_Set` _allcells _array_index _structout))
    (set `self.AnimateHasMadeChange` true)))

(event `Key|T`
  (params (Key :type "Key Structure"))
  ;[0 0 0] Hides all elements and animates in to state set by editor or randomisation above
  (:`Pressed`
    (`self.AnimateIn`)))

(event `self.ReceiveTick`
  (params (DeltaSeconds :type "Float (single-precision)"))
  (if (`self.AnimateHasMadeChange`)
    (`self.UpdateView`)
    (set `self.AnimateHasMadeChange` false)))

(fn `AnimateIn`
  (locals (CurrentAnimateInStep :type "Array of Integer"))
  (set `self.CurrentAnimateInIndex` 0)
  (for _array_element (`self.AllCells`)
    (`SceneComponent.SetVisibility` (`.Object_4_22610DB1694CC3235CE446A6404399D0` (break `/Game/blueprints/SObjectSetCell` _array_element)) false false))
  (`KismetSystemLibrary.K2_SetTimer` null "AnimateInStep" 0.01 true))

(fn `AnimateInStep`
  (bind _currentanimateinindex (`self.CurrentAnimateInIndex`))
  (bind _allcells (`self.AllCells`))
  (bind (_visible _object) (break `/Game/blueprints/SObjectSetCell` (`|GetArrayItem` _allcells _currentanimateinindex)))
  (`SceneComponent.SetVisibility` _object _visible false)
  (bind _output_get (set `self.CurrentAnimateInIndex` (+ _currentanimateinindex 1)))
  (if (>= _output_get (`KismetArrayLibrary.Array_Length` _allcells))
    (`KismetSystemLibrary.K2_ClearTimer` null "AnimateInStep")))

(fn `ClearSpawned`
  (bind _spawnedobjects (`self.SpawnedObjects`))
  (for _array_element _spawnedobjects
    (`ActorComponent.K2_DestroyComponent` _array_element)
    (`KismetArrayLibrary.Array_Clear` _spawnedobjects :!label _label))
  (goto _label))

(fn `SetBoundsSize`
  (bind (_areasize_x _areasize_y _areasize_z) (`KismetMathLibrary.BreakVector` (`self.AreaSize`)))
  (bind _bounds (`self.Bounds`))
  (bind _returnvalue (* _areasize_x 0.5))
  (bind _returnvalue_2 (* _areasize_z 0.5))
  (bind _returnvalue_3 (* _areasize_y 0.5))
  (`BoxComponent.SetBoxExtent` _bounds (`KismetMathLibrary.MakeVector` _returnvalue _returnvalue_3 _returnvalue_2) true)
  (`SceneComponent.K2_SetRelativeTransform` _bounds (`KismetMathLibrary.MakeTransform` (`KismetMathLibrary.MakeVector` (* _returnvalue -1.0) (* _returnvalue_3 -1.0) _returnvalue_2)) false true))

(fn `SpawnGridOfMeshAt`
  (params (Mesh :type "StaticMesh Object Reference") (Location :type "Vector Structure") (AvailableSpace :type "Vector Structure") (MaxItemsHigh :type Integer) (SendItemsDeep :type Boolean) (MaxItemsAcross :type Integer) (Variance :type "Float (double-precision)") (Density :type "Float (double-precision)") (RandomSeed :type Integer))
  (returns (GridSize :type "Vector Structure") (SpawnedCellList :type "Array of /Game/blueprints/SObjectSetCell Structure"))
  (locals (MeshSize :type "Vector Structure") (SpawnedMeshList :type "Array of StaticMeshComponent Object Reference") (StepsX :type Integer) (StepsY :type Integer) (StepsZ :type Integer) (Origin :type "Vector Structure") (PositionMaxVariation :type "Float (double-precision)") (XYPresence :type "Array of Boolean") (GridRandomSource :type "RandomStream Structure") (SpawnedCells :type "Array of /Game/blueprints/SObjectSetCell Structure"))
  (bind (_meshsize_x _meshsize_y _meshsize_z) (`KismetMathLibrary.BreakVector` (`local.MeshSize`)))
  (bind _meshsize_x_2 (`KismetMathLibrary.BreakVector` (`local.MeshSize`)))
  (bind _stepsy (`local.StepsY`))
  (bind _positionmaxvariation (`local.PositionMaxVariation`))
  (bind _positionmaxvariation_2 (`local.PositionMaxVariation`))
  (bind _positionmaxvariation_3 (`local.PositionMaxVariation`))
  (bind _stepsy_2 (`local.StepsY`))
  (bind _objectgap (`self.ObjectGap`))
  (bind _stepsz (`local.StepsZ`))
  (bind (_meshsize_x_3 _meshsize_y_2 _meshsize_z_2) (`KismetMathLibrary.BreakVector` (`local.MeshSize`)))
  (bind _gridrandomsource (`local.GridRandomSource`))
  (bind _stepsz_2 (`local.StepsZ`))
  (bind _objectgap_2 (`self.ObjectGap`))
  (bind (_min _max) (break `Box` (`StaticMesh.GetBoundingBox` Mesh)))
  (bind _returnvalue (`KismetMathLibrary.MakeRotator` 0.0 0.0 (`KismetMathLibrary.RandomFloatInRangeFromStream` (* _positionmaxvariation_2 -3.0) (* _positionmaxvariation_2 3.0) (`local.GridRandomSource`))))
  (bind _returnvalue_2 (`KismetMathLibrary.MakeVector` (`KismetMathLibrary.RandomFloatInRangeFromStream` (* _positionmaxvariation_3 -1.0) _positionmaxvariation_3 _gridrandomsource) (`KismetMathLibrary.RandomFloatInRangeFromStream` (* _positionmaxvariation -1.0) _positionmaxvariation _gridrandomsource)))
  (`|ExecutionSequence`
    (:`then_0`
      ;[0 0 0] Measure the chosen Mesh
      (bind _returnvalue_3 (`AddComponent|NODE_AddStaticMeshComponent-1`))
      (`StaticMeshComponent.SetStaticMesh` _returnvalue_3 Mesh)
      (set `local.MeshSize` (- _max _min))
      (`ActorComponent.K2_DestroyComponent` _returnvalue_3))
    (:`then_1`
      ;[0 0 0] Initialise Variables
      (`/Game/blueprints/BPFL_Helpers.GM_Random_PickOrUseSeed` RandomSeed (`local.GridRandomSource`))
      (set `local.Origin` Location)
      (if (>= (`KismetMathLibrary.RandomFloatFromStream` (`local.GridRandomSource`)) (- 1.0 Density))
        (set `local.StepsZ` MaxItemsHigh)
        (else
          (set `local.StepsZ` (`KismetMathLibrary.RandomIntegerInRangeFromStream` 1 MaxItemsHigh (`local.GridRandomSource`)))))
      (set `local.StepsY` (`KismetMathLibrary.RandomIntegerInRangeFromStream` 1 MaxItemsAcross (`local.GridRandomSource`)))
      (if SendItemsDeep
        (set `local.StepsX` (`KismetMathLibrary.FFloor` (/ (.x AvailableSpace) (+ _meshsize_x_2 (`self.ObjectGap`)))))
        (else
          (set `local.StepsX` 1)))
      (set `local.PositionMaxVariation` (* Variance (/ (`self.ObjectGap`) 2.0))))
    (:`then_2`
      ;[0 0 0] initialising a 3d array with visible/invisible booleans for presence/absence of objects
      (`KismetArrayLibrary.Array_Clear` (`local.SpawnedCells`))
      (for _index (range _stepsy_2)
        (for _index_2 (range (`local.StepsX`))
          (for _index_3 (range _stepsz)
            (bind _index_4 (`/Game/blueprints/BPFL_Helpers.GM_Array_From3dTo1dIndex` _index_2 _index _index_3 _stepsy_2 _stepsz))
            (if (== _index_3 0)
              ;[0 0 0] Calculate visibility on bottom row
              (`KismetArrayLibrary.Array_Set` (`local.SpawnedCells`) _index_4 (make `/Game/blueprints/SObjectSetCell` (>= (`KismetMathLibrary.RandomFloatFromStream` (`local.GridRandomSource`)) (- 1.0 Density))) true)
              (else
                ;[0 0 0] This is above the bottom row, calculate visibility based on row below
                (bind _index_5 (`/Game/blueprints/BPFL_Helpers.GM_Array_From3dTo1dIndex` _index_2 _index (- _index_3 1) (`local.StepsY`) (`local.StepsZ`)))
                (if (`.Visible_1_F28072AAD3463772E651679B665C4602` (break `/Game/blueprints/SObjectSetCell` (`|GetArrayItem` (`local.SpawnedCells`) _index_5)))
                  ;[0 0 0] Below is visible - decide whether to hide
                  (`KismetArrayLibrary.Array_Set` (`local.SpawnedCells`) _index_4 (make `/Game/blueprints/SObjectSetCell` (>= (`KismetMathLibrary.RandomFloatFromStream` (`local.GridRandomSource`)) (- 1.0 Density))) true)
                  (else
                    ;[0 0 0] Below is hidden. Hide this too
                    (`KismetArrayLibrary.Array_Set` (`local.SpawnedCells`) _index_4 (make `/Game/blueprints/SObjectSetCell` false) true)))))))))
    (:`then_3`
      (for _index_6 (range _stepsy)
        (for _index_7 (range (`local.StepsX`))
          (for _index_8 (range _stepsz_2)
            (bind _index_9 (`/Game/blueprints/BPFL_Helpers.GM_Array_From3dTo1dIndex` _index_7 _index_6 _index_8 _stepsy _stepsz_2))
            (bind _returnvalue_4 (+ (`KismetMathLibrary.MakeVector` (* (* _index_7 (+ _meshsize_x _objectgap_2)) -1.0) (* (* _index_6 (+ _meshsize_y _objectgap_2)) -1.0) (* _index_8 _meshsize_z)) (`local.Origin`)))
            ;[0 0 0] Add the mesh at location
            (bind _spawnedmesh (`self.SpawnMeshAt` Mesh (+ _returnvalue_2 _returnvalue_4)))
            (`SceneComponent.K2_SetRelativeRotation` _spawnedmesh _returnvalue false false)
            (bind _output (`|GetArrayItem` (`local.SpawnedCells`) _index_9))
            (bind _visible (break `/Game/blueprints/SObjectSetCell` _output))
            ;[0 0 0] If this object shouldn't be there set hidden
            (`SceneComponent.SetVisibility` _spawnedmesh _visible false)
            (setmembers `/Game/blueprints/SObjectSetCell` :`StructRef` _output :`Visible` _visible :`Object` _spawnedmesh :`Origin` _returnvalue_4 :`OffsetPosition` _returnvalue_2 :`OffsetRotation` _returnvalue :`Size` (`local.MeshSize`))))))
    (:`then_4`
      ;[0 0 0] Calculate used size and output with list of meshes
      (return (`KismetMathLibrary.MakeVector` (* (+ _meshsize_x_3 _objectgap) (`local.StepsX`)) (* (+ _meshsize_y_2 _objectgap) (`local.StepsY`)) (* _meshsize_z_2 (`local.StepsZ`))) (`local.SpawnedCells`)))))

(fn `SpawnMeshAt`
  (params (Mesh :type "StaticMesh Object Reference") (Location :type "Vector Structure"))
  (returns (SpawnedMesh :type "StaticMeshComponent Object Reference") (MeshSize :type "Vector Structure"))
  (bind (_min _max) (break `Box` (`StaticMesh.GetBoundingBox` Mesh)))
  (bind _returnvalue (- _max _min))
  (bind _returnvalue_2 (`AddComponent|NODE_AddStaticMeshComponent-0` :`RelativeTransform` (`KismetMathLibrary.Conv_VectorToTransform` (- Location (`KismetMathLibrary.MakeVector` (/ (.x _returnvalue) 2.0) (/ (.y _returnvalue) 2.0))))))
  (`StaticMeshComponent.SetStaticMesh` _returnvalue_2 Mesh)
  (return _returnvalue_2 _returnvalue))

(fn `UpdateView`
  (for _array_element (`self.AllCells`)
    (bind (_visible _object _origin _offsetposition _offsetrotation) (break `/Game/blueprints/SObjectSetCell` _array_element))
    (`SceneComponent.SetVisibility` _object _visible false)
    (`SceneComponent.K2_SetRelativeRotation` _object _offsetrotation false false)
    (`SceneComponent.K2_SetRelativeLocation` _object (+ _origin _offsetposition) false true)))

(fn `UserConstructionScript`
  (locals (SpawnPossible :type Boolean) (SpawnIndex :type Integer) (CurrentSpawnLocation :type "Vector Structure"))
  (bind _possibleobjects (`self.PossibleObjects`))
  (bind (_currentspawnlocation_x _currentspawnlocation_y _currentspawnlocation_z) (`KismetMathLibrary.BreakVector` (`local.CurrentSpawnLocation`)))
  (bind (_areasize_x _areasize_y _areasize_z) (`KismetMathLibrary.BreakVector` (`self.AreaSize`)))
  (bind (_currentspawnlocation_x_2 _currentspawnlocation_y_2 _currentspawnlocation_z_2) (`KismetMathLibrary.BreakVector` (`local.CurrentSpawnLocation`)))
  (bind _currentspawnlocation (`local.CurrentSpawnLocation`))
  (bind (_areasize_x_2 _areasize_y_2) (`KismetMathLibrary.BreakVector` (`self.AreaSize`)))
  (bind (_mesh _stackable _deep _across) (break `/Game/blueprints/SObjectInfo` (`|GetArrayItem` _possibleobjects (`KismetMathLibrary.RandomIntegerInRangeFromStream` 0 (- (`KismetArrayLibrary.Array_Length` _possibleobjects) 1) (`self.RandomSource`)))))
  (`|ExecutionSequence`
    (:`then_0`
      (bind _randomseedinuse (`/Game/blueprints/BPFL_Helpers.GM_Random_PickOrUseSeed` (`self.RandomSeed`) (`self.RandomSource`)))
      (set `self.RandomSeedInUse` _randomseedinuse))
    (:`then_1`
      (`self.SetBoundsSize`))
    (:`then_2`
      (if (`self.IsActive`)
        (`self.ClearSpawned`)
        (set `local.CurrentSpawnLocation` (`KismetMathLibrary.MakeVector` 0.0 (* (`self.ObjectGap`) -1.0)))
        (bind _output_get (set `local.SpawnPossible` true))
        (set `local.SpawnIndex` 0)
        (while _output_get
          (bind (_gridsize _spawnedcelllist) (`self.SpawnGridOfMeshAt` _mesh _currentspawnlocation (`KismetMathLibrary.MakeVector` _areasize_x (- _areasize_y (`KismetMathLibrary.Abs` (.y _currentspawnlocation))) _areasize_z) _stackable _deep _across (`self.Variance`) (`self.Density`) (+ (`self.RandomSeedInUse`) (`local.SpawnIndex`))))
          (set `local.SpawnIndex` (+ (`local.SpawnIndex`) 1))
          (bind _output_get_2 (set `local.CurrentSpawnLocation` (`KismetMathLibrary.MakeVector` _currentspawnlocation_x_2 (- _currentspawnlocation_y_2 (.y _gridsize)) _currentspawnlocation_z_2)))
          (if (< (.y _output_get_2) (* _areasize_y_2 -1.0))
            (for _array_element _spawnedcelllist
              (`ActorComponent.K2_DestroyComponent` (`.Object_4_22610DB1694CC3235CE446A6404399D0` (break `/Game/blueprints/SObjectSetCell` _array_element))))
            (set `local.SpawnPossible` false)
            (else
              (`KismetArrayLibrary.Array_Append` (`self.AllCells`) _spawnedcelllist)
              (set `local.CurrentSpawnLocation` (`KismetMathLibrary.MakeVector` _currentspawnlocation_x (- _currentspawnlocation_y (`self.ObjectGap`)) _currentspawnlocation_z)))))))))