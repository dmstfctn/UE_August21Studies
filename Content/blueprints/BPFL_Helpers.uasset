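; BPFL_Helpers is a Blueprint function library of grid-indexing and random-seed helpers.
; Two functions convert between 3D coordinates and a flat array index, with Z varying fastest, using the Y and Z dimensions.
; The seed helper seeds a Random Stream with the given positive seed, otherwise a random one, returning the stream and seed.
; The pure random node feeds both seeding and return separately, so a random seed's reported value can differ.
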(fn `GM_Array_From1dTo3dIndex`
  (params (Index :type Integer) (DY :type Integer) (DZ :type Integer))
  (returns (X :type Integer) (Y :type Integer) (Z :type Integer))
  (bind _returnvalue (mod Index DZ))
  (bind _returnvalue_2 (- Index _returnvalue))
  (bind _returnvalue_3 (mod (/ _returnvalue_2 DZ) DY))
  (return (/ (- _returnvalue_2 (* DZ _returnvalue_3)) (* DZ DY)) _returnvalue_3 _returnvalue))

(fn `GM_Array_From3dTo1dIndex`
  (params (X :type Integer) (Y :type Integer) (Z :type Integer) (DY :type Integer) (DZ :type Integer))
  (returns (Index :type Integer))
  (return (+ (* (* X DY) DZ) (* Y DZ) Z 0)))

(fn `GM_Random_PickOrUseSeed`
  (params (RandomSeed :type Integer) (RandomSourceIn :type "RandomStream Structure (by ref)"))
  (returns (RandomSeedInUse :type Integer) (RandomSourceOut :type "RandomStream Structure"))
  (bind _returnvalue (select `int` (`KismetMathLibrary.Clamp` RandomSeed 0 1) :`0` (`KismetMathLibrary.RandomInteger` 100000) :`1` RandomSeed))
  (`KismetMathLibrary.SetRandomStreamSeed` RandomSourceIn _returnvalue)
  (return _returnvalue RandomSourceIn))