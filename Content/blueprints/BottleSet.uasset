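; BottleSet is a placeable actor that fills a rectangular area with a grid of RandomBottle actors.
; The construction script sizes Bounds from AreaDepth and AreaWidth and hides the preview Cube.
; BeginPlay fits rows and columns by BottleSize, spawning attached bottles with slight position and yaw jitter.
; All bottles share one type ID, randomized when BottleTypeID is zero or less, and are destroyed with the set.
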(event `self.ReceiveBeginPlay`
  (bind _bottlesize (`self.BottleSize`))
  (bind _bottlesize_2 (`self.BottleSize`))
  (bind _bottletypeid (`self.BottleTypeID`))
  (bind _returnvalue (/ _bottlesize 2.0))
  (`|ExecutionSequence`
    (:`then_0`
      (set `self.UseBottleTypeID` (select `int` (`KismetMathLibrary.Clamp` _bottletypeid 0 1) :`0` (`KismetMathLibrary.RandomInteger` 100000) :`1` _bottletypeid)))
    (:`then_1`
      (for _index (range (`KismetMathLibrary.FFloor` (/ (* (.y (`BoxComponent.GetScaledBoxExtent` (`self.Bounds`))) 2.0) _bottlesize_2)))
        (for _index_2 (range (`KismetMathLibrary.FFloor` (/ (* (.x (`BoxComponent.GetScaledBoxExtent` (`self.Bounds`))) 2.0) _bottlesize_2)))
          (bind _returnvalue_2 (`|SpawnActorFromClass` "/Game/blueprints/RandomBottle.RandomBottle_C" (`KismetMathLibrary.MakeTransform` (+ (`KismetMathLibrary.MakeVector` (* (+ (* _index_2 _bottlesize) _returnvalue) -1.0) (- (* (* _index _bottlesize) -1.0) _returnvalue) (* (.z (`BoxComponent.GetScaledBoxExtent` (`self.Bounds`))) 0.0)) (`KismetMathLibrary.MakeVector` (`KismetMathLibrary.RandomFloatInRange` -1.0 1.0) (`KismetMathLibrary.RandomFloatInRange` -1.0 1.0))) (`KismetMathLibrary.MakeRotator` 0.0 0.0 (`KismetMathLibrary.RandomFloatInRange` -15.0 15.0))) "AdjustIfPossibleButAlwaysSpawn" "OverrideRootScale" null (`self.UseBottleTypeID`) null))
          (`self.K2_AttachToActor` _returnvalue_2 (`ActorComponent.GetOwner` (`self.DefaultSceneRoot`)) "None" "KeepRelative" "KeepRelative" "KeepRelative" false)
          (`KismetArrayLibrary.Array_Add` (`self.SpawnedBottles`) _returnvalue_2))))))

(event `self.ReceiveDestroyed`
  (for _array_element (`self.SpawnedBottles`)
    (`self.K2_DestroyActor` _array_element)))

(fn `UserConstructionScript`
  (bind _bounds (`self.Bounds`))
  (bind _areawidth (`self.AreaWidth`))
  (bind _areadepth (`self.AreaDepth`))
  (bind _cube (`self.Cube`))
  (bind _returnvalue (`KismetMathLibrary.MakeVector` _areadepth _areawidth 5.0))
  (bind _returnvalue_2 (`KismetMathLibrary.MakeTransform` (`KismetMathLibrary.MakeVector` (* _areadepth -1.0) (* _areawidth -1.0) 5.0)))
  (`BoxComponent.SetBoxExtent` _bounds _returnvalue true)
  (`SceneComponent.K2_SetRelativeTransform` _bounds _returnvalue_2 false true)
  (if false
    (`SceneComponent.K2_SetRelativeTransform` _cube _returnvalue_2 false true)
    (`SceneComponent.SetRelativeScale3D` _cube (/ _returnvalue (50.0 50.0 50.0)))
    (else
      (`SceneComponent.SetVisibility` (`self.Cube`) false false))))