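; Procedural prop set that fills a box area at construction with randomized grids of static meshes from PossibleObjects.
; The construction script seeds a random stream and lays grids along negative Y, separated by ObjectGap, destroying the one that overflows.
; SpawnGridOfMeshAt sizes each grid from mesh bounds and stacking limits, jittering position and yaw by Variance.
; A flattened 3D boolean array hides items by Density, hiding anything above a hidden item.
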(event `self.ReceiveBeginPlay`)

(fn `From1dTo3dIndex`
  (params (index :type Integer) (dY :type Integer) (dZ :type Integer))
  (returns (x :type Integer) (y :type Integer) (z :type Integer))
  (bind _returnvalue (mod index dZ))
  (bind _returnvalue_2 (- index _returnvalue))
  (bind _returnvalue_3 (mod (/ _returnvalue_2 dZ) dY))
  (return (/ (- _returnvalue_2 (* dZ _returnvalue_3)) (* dZ dY)) _returnvalue_3 _returnvalue))

(fn `From3dTo1dIndex`
  (params (x :type Integer) (y :type Integer) (z :type Integer) (dY :type Integer) (dZ :type Integer))
  (returns (index :type Integer))
  (return (+ (* (* x dY) dZ) (* y dZ) z 0)))

(fn `SpawnGridOfMeshAt`
  (params (Mesh :type "StaticMesh Object Reference") (Location :type "Vector Structure") (AvailableSpace :type "Vector Structure") (MaxItemsHigh :type Integer) (SendItemsDeep :type Boolean) (MaxItemsAcross :type Integer) (Variance :type "Float (double-precision)") (Density :type "Float (double-precision)") (RandomSeed :type Integer))
  (returns (GridSize :type "Vector Structure") (SpawnedMeshes :type "Array of StaticMeshComponent Object Reference"))
  (locals (MeshSize :type "Vector Structure") (SpawnedMeshList :type "Array of StaticMeshComponent Object Reference") (StepsX :type Integer) (StepsY :type Integer) (StepsZ :type Integer) (Origin :type "Vector Structure") (PositionMaxVariation :type "Float (double-precision)") (XYPresence :type "Array of Boolean") (GridRandomSource :type "RandomStream Structure"))
  (bind (_meshsize_x _meshsize_y _meshsize_z) (`KismetMathLibrary.BreakVector` (`local.MeshSize`)))
  (bind _meshsize_x_2 (`KismetMathLibrary.BreakVector` (`local.MeshSize`)))
  (bind _stepsy (`local.StepsY`))
  (bind _positionmaxvariation (`local.PositionMaxVariation`))
  (bind _positionmaxvariation_2 (`local.PositionMaxVariation`))
  (bind _positionmaxvariation_3 (`local.PositionMaxVariation`))
  (bind _stepsy_2 (`local.StepsY`))
  (bind _objectgap (`self.ObjectGap`))
  (bind _xypresence (`local.XYPresence`))
  (bind _stepsz (`local.StepsZ`))
  (bind (_meshsize_x_3 _meshsize_y_2 _meshsize_z_2) (`KismetMathLibrary.BreakVector` (`local.MeshSize`)))
  (bind _gridrandomsource (`local.GridRandomSource`))
  (bind _stepsz_2 (`local.StepsZ`))
  (bind _objectgap_2 (`self.ObjectGap`))
  (bind (_min _max) (break `Box` (`StaticMesh.GetBoundingBox` Mesh)))
  (`|ExecutionSequence`
    (:`then_0`
      ;[0 0 0] Measure the chosen Mesh
      (bind _returnvalue (`AddComponent|NODE_AddStaticMeshComponent-5`))
      (`StaticMeshComponent.SetStaticMesh` _returnvalue Mesh)
      (set `local.MeshSize` (- _max _min))
      (`ActorComponent.K2_DestroyComponent` _returnvalue))
    (:`then_1`
      ;[0 0 0] Initialise Variables
      (`KismetMathLibrary.SetRandomStreamSeed` (`local.GridRandomSource`) (select `int` (`KismetMathLibrary.Clamp` RandomSeed 0 1) :`0` (`KismetMathLibrary.RandomInteger` 100000) :`1` RandomSeed))
      (set `local.Origin` Location)
      (if (>= (`KismetMathLibrary.RandomFloatFromStream` (`local.GridRandomSource`)) (- 1.0 Density))
        (set `local.StepsZ` MaxItemsHigh)
        (else
          (set `local.StepsZ` (`KismetMathLibrary.RandomIntegerInRangeFromStream` 1 MaxItemsHigh (`local.GridRandomSource`)))))
      (set `local.StepsY` (`KismetMathLibrary.RandomIntegerInRangeFromStream` 1 MaxItemsAcross (`local.GridRandomSource`)))
      (if SendItemsDeep
        (set `local.StepsX` (`KismetMathLibrary.FFloor` (/ (.x AvailableSpace) (+ _meshsize_x_2 (`self.ObjectGap`)))))
        (else
          (set `local.StepsX` 1)))
      (set `local.PositionMaxVariation` (* Variance (/ (`self.ObjectGap`) 2.0))))
    (:`then_2`
      ;[0 0 0] initialising a 3d array with visible/invisible booleans for presence/absence of objects
      (`KismetArrayLibrary.Array_Clear` (`local.XYPresence`))
      (for _index (range _stepsy_2)
        (for _index_2 (range (`local.StepsX`))
          (for _index_3 (range _stepsz)
            (bind _index_4 (`/Game/blueprints/BPFL_Helpers.GM_Array_From3dTo1dIndex` _index_2 _index _index_3 _stepsy_2 _stepsz))
            (if (== _index_3 0)
              ;[0 0 0] Calculate visibility on bottom row
              (`KismetArrayLibrary.Array_Set` _xypresence _index_4 (>= (`KismetMathLibrary.RandomFloatFromStream` (`local.GridRandomSource`)) (- 1.0 Density)) true)
              (else
                ;[0 0 0] This is above the bottom row, calculate visibility based on row below
                (bind _index_5 (`/Game/blueprints/BPFL_Helpers.GM_Array_From3dTo1dIndex` _index_2 _index (- _index_3 1) (`local.StepsY`) (`local.StepsZ`)))
                (if (`|GetArrayItem` _xypresence _index_5)
                  ;[0 0 0] Below is visible - decide whether to hide
                  (`KismetArrayLibrary.Array_Set` _xypresence _index_4 (>= (`KismetMathLibrary.RandomFloatFromStream` (`local.GridRandomSource`)) (- 1.0 Density)) true)
                  (else
                    ;[0 0 0] Below is hidden. Hide this too
                    (`KismetArrayLibrary.Array_Set` _xypresence _index_4 false true)))))))))
    (:`then_3`
      (for _index_6 (range _stepsy)
        (for _index_7 (range (`local.StepsX`))
          (for _index_8 (range _stepsz_2)
            (bind _index_9 (`/Game/blueprints/BPFL_Helpers.GM_Array_From3dTo1dIndex` _index_7 _index_6 _index_8 _stepsy _stepsz_2))
            ;[0 0 0] Add the mesh at location and store reference
            (bind _spawnedmesh (`self.SpawnMeshAt` Mesh (+ (`KismetMathLibrary.MakeVector` (* (* _index_7 (+ _meshsize_x _objectgap_2)) -1.0) (* (* _index_6 (+ _meshsize_y _objectgap_2)) -1.0) (* _index_8 _meshsize_z)) (`local.Origin`) (`KismetMathLibrary.MakeVector` (`KismetMathLibrary.RandomFloatInRangeFromStream` (* _positionmaxvariation_3 -1.0) _positionmaxvariation_3 _gridrandomsource) (`KismetMathLibrary.RandomFloatInRangeFromStream` (* _positionmaxvariation -1.0) _positionmaxvariation _gridrandomsource)))))
            (`SceneComponent.K2_SetRelativeRotation` _spawnedmesh (`KismetMathLibrary.MakeRotator` 0.0 0.0 (`KismetMathLibrary.RandomFloatInRangeFromStream` (* _positionmaxvariation_2 -3.0) (* _positionmaxvariation_2 3.0) (`local.GridRandomSource`))) false false)
            (`KismetArrayLibrary.Array_Add` (`local.SpawnedMeshList`) _spawnedmesh)
            ;[0 0 0] If this object shouldn't be there set hidden
            (`SceneComponent.SetVisibility` _spawnedmesh (`|GetArrayItem` (`local.XYPresence`) _index_9) false)))))
    (:`then_4`
      ;[0 0 0] Calculate used size and output with list of meshes
      (return (`KismetMathLibrary.MakeVector` (* (+ _meshsize_x_3 _objectgap) (`local.StepsX`)) (* (+ _meshsize_y_2 _objectgap) (`local.StepsY`)) (* _meshsize_z_2 (`local.StepsZ`))) (`local.SpawnedMeshList`)))))

(fn `SpawnMeshAt`
  (params (Mesh :type "StaticMesh Object Reference") (Location :type "Vector Structure"))
  (returns (SpawnedMesh :type "StaticMeshComponent Object Reference") (MeshSize :type "Vector Structure"))
  (bind (_min _max) (break `Box` (`StaticMesh.GetBoundingBox` Mesh)))
  (bind _returnvalue (- _max _min))
  (bind _returnvalue_2 (`AddComponent|NODE_AddStaticMeshComponent-4` :`RelativeTransform` (`KismetMathLibrary.Conv_VectorToTransform` (- Location (`KismetMathLibrary.MakeVector` (/ (.x _returnvalue) 2.0) (/ (.y _returnvalue) 2.0))))))
  (`StaticMeshComponent.SetStaticMesh` _returnvalue_2 Mesh)
  (return _returnvalue_2 _returnvalue))

(fn `UserConstructionScript`
  (bind _possibleobjects (`self.PossibleObjects`))
  (bind (_areasize_x _areasize_y _areasize_z) (`KismetMathLibrary.BreakVector` (`self.AreaSize`)))
  (bind _bounds (`self.Bounds`))
  (bind _randomseed (`self.RandomSeed`))
  (bind (_currentspawnlocation_x _currentspawnlocation_y _currentspawnlocation_z) (`KismetMathLibrary.BreakVector` (`self.CurrentSpawnLocation`)))
  (bind (_areasize_x_2 _areasize_y_2 _areasize_z_2) (`KismetMathLibrary.BreakVector` (`self.AreaSize`)))
  (bind (_currentspawnlocation_x_2 _currentspawnlocation_y_2 _currentspawnlocation_z_2) (`KismetMathLibrary.BreakVector` (`self.CurrentSpawnLocation`)))
  (bind _currentspawnlocation (`self.CurrentSpawnLocation`))
  (bind (_areasize_x_3 _areasize_y_3) (`KismetMathLibrary.BreakVector` (`self.AreaSize`)))
  (bind _returnvalue (* _areasize_x 0.5))
  (bind _returnvalue_2 (* _areasize_z 0.5))
  (bind _returnvalue_3 (* _areasize_y 0.5))
  (bind _returnvalue_4 (select `int` (`KismetMathLibrary.Clamp` _randomseed 0 1) :`0` (`KismetMathLibrary.RandomInteger` 100000) :`1` _randomseed))
  (bind (_mesh _stackable _deep _across) (break `/Game/blueprints/SObjectInfo` (`|GetArrayItem` _possibleobjects (`KismetMathLibrary.RandomIntegerInRangeFromStream` 0 (- (`KismetArrayLibrary.Array_Length` _possibleobjects) 1) (`self.RandomSource`)))))
  (`|ExecutionSequence`
    (:`then_0`
      (`KismetMathLibrary.SetRandomStreamSeed` (`self.RandomSource`) _returnvalue_4)
      (set `self.RandomSeedInUse` _returnvalue_4))
    (:`then_1`
      (`BoxComponent.SetBoxExtent` _bounds (`KismetMathLibrary.MakeVector` _returnvalue _returnvalue_3 _returnvalue_2) true)
      (`SceneComponent.K2_SetRelativeTransform` _bounds (`KismetMathLibrary.MakeTransform` (`KismetMathLibrary.MakeVector` (* _returnvalue -1.0) (* _returnvalue_3 -1.0) _returnvalue_2)) false true))
    (:`then_2`
      (set `self.CurrentSpawnLocation` (`KismetMathLibrary.MakeVector` 0.0 (* (`self.ObjectGap`) -1.0)))
      (bind _output_get (set `self.SpawnPossible` true))
      (set `self.SpawnIndex` 0)
      (while _output_get
        (bind (_gridsize _spawnedmeshes) (`self.SpawnGridOfMeshAt` _mesh _currentspawnlocation (`KismetMathLibrary.MakeVector` _areasize_x_2 (- _areasize_y_2 (`KismetMathLibrary.Abs` (.y _currentspawnlocation))) _areasize_z_2) _stackable _deep _across (`self.Variance`) (`self.Density`) (+ (`self.RandomSeedInUse`) (`self.SpawnIndex`))))
        (set `self.SpawnIndex` (+ (`self.SpawnIndex`) 1))
        (bind _output_get_2 (set `self.CurrentSpawnLocation` (`KismetMathLibrary.MakeVector` _currentspawnlocation_x_2 (- _currentspawnlocation_y_2 (.y _gridsize)) _currentspawnlocation_z_2)))
        (if (< (.y _output_get_2) (* _areasize_y_3 -1.0))
          (for _array_element _spawnedmeshes
            (`ActorComponent.K2_DestroyComponent` _array_element))
          (set `self.SpawnPossible` false)
          (else
            (`KismetArrayLibrary.Array_Append` (`self.SpawnedObjects`) _spawnedmeshes)
            (set `self.CurrentSpawnLocation` (`KismetMathLibrary.MakeVector` _currentspawnlocation_x (- _currentspawnlocation_y (`self.ObjectGap`)) _currentspawnlocation_z))))))))